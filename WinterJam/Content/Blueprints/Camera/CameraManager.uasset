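; CameraManager is an actor that owns the game's main cine camera and keeps it drifting through the world.
; On BeginPlay, Spawn sets the first player controller's view target to the camera's owner.
; Each Tick, Move offsets the CineCamera in world space by DefaultVelocity scaled by delta time, without sweeping.
; GetMainCamera exposes the camera to other code.
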(event EventBeginPlay
  (Spawn|Spawn))

(event Collision|EventActorBeginOverlap
  (params (OtherActor :type Actor%20Object%20Reference)))

(event EventTick
  (params (DeltaSeconds :type Float%20%28single-precision%29))
  (Move|Move))

(fn ConstructionScript)

(fn Spawn
  (Game|Player|SetViewTargetwithBlend (Game|GetPlayerController 0) (Components|GetOwner (Variables|Default|GetCineCamera)) 0.0 "VTBlend_Linear" 0.0 false))

(fn GetMainCamera
  (return (Variables|Default|GetCineCamera)))

(fn Move
  (Transformation|AddWorldOffset (Variables|Default|GetCineCamera) (* (Variables|Default|GetDefaultVelocity) (Utilities|Time|GetWorldDeltaSeconds)) false false))