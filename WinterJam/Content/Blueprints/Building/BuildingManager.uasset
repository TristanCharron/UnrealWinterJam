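; Building manager that stacks randomly chosen buildings vertically above a first building while the game is running.
; It reacts to the GameManager's game start dispatcher: In Game resets the count and list, spawns immediately and starts a looping timer, while Before and End Game stop it.
; Each spawn is offset by the first building's height times the count.
; Resetting clears references without destroying spawned actors.
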(event Custom|OnGameStart
  (params (NextGameState :type EGameStates%20Enum :default "NewEnumerator0"))
  (switch Utilities|FlowControl|Switch|SwitchonEGameStates NextGameState
    (:NewEnumerator0
      (CallFunction|StopSpawn :!label _label))
    (:NewEnumerator1
      (bind _returnvalue (Utilities|Time|SetTimerbyFunctionName self "Spawn" 5.0 true))
      (Variables|Default|SetSpawnTimeHandler _returnvalue)
      (CallFunction|ResetBuildings)
      (CallFunction|Spawn))
    (:NewEnumerator2
      (goto _label))))

(event EventBeginPlay
  (EventDispatchers|BindEventtoGameStartDispatcher (CallFunction|GetGameManager) (delegate Custom|OnGameStart)))

(event Collision|EventActorBeginOverlap
  (params (OtherActor :type Actor%20Object%20Reference)))

(event EventTick
  (params (DeltaSeconds :type Float%20%28single-precision%29)))

(fn ConstructionScript)

(fn Spawn
  (bind _firstbuilding (Variables|Default|GetFirstBuilding))
  (bind _output_get (Variables|Default|SetNbBuildingsLoaded (+ (Variables|Default|GetNbBuildingsLoaded) 1)))
  (bind _returnvalue (Game|SpawnActorfromClass (Utilities|Array|Get(acopy) (Variables|Default|GetBuildingClassList) (Math|Random|RandomIntegerinRange 0 (- (Utilities|Array|Length (Variables|Default|GetBuildingClassList)) 1))) (Math|Transform|MakeTransform (+ (Transformation|GetActorLocation _firstbuilding) (* (Math|Vector|MakeVector 0.0 0.0 (* (.z (.BoxExtent (Collision|GetActorBounds (Variables|Default|GetFirstBuilding) true))) 2.0)) _output_get)) (Transformation|GetActorRotation _firstbuilding) (Variables|Default|GetBuildingScale)) "Undefined" 0 0))
  (Utilities|Array|Add (Variables|Default|GetBuildingSpawnedList) _returnvalue))

(fn ResetBuildings
  (Variables|Default|SetNbBuildingsLoaded 0)
  (Utilities|Array|Clear (Variables|Default|GetBuildingSpawnedList)))

(fn StopSpawn
  (if (Utilities|Time|IsValidTimerHandle (Variables|Default|GetSpawnTimeHandler))
    (Utilities|Time|ClearandInvalidateTimerbyHandle (Variables|Default|GetSpawnTimeHandler))))