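; BP_Building is a building actor that randomly populates its three sides with nacelles at startup.
; BeginPlay groups child-actor slots into four per side, and SpawnNacelle uses a Set to draw two distinct indices for each.
; It spawns BP_Nacelle at each slot's Arrow and attaches it to Cylinder, but writes the slot's ActorRef before that spawn.
; The RotateBuilding timeline would yaw Cylinder but is never triggered, and IsSlotEmpty is unused.
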(event EventBeginPlay
  (Utilities|FlowControl|Sequence
    (:then_1
      (Variables|Default|SetSide1 (Utilities|Array|MakeArray (Variables|Default|GetS1-3) (Variables|Default|GetS1-4) (Variables|Default|GetS1-1) (Variables|Default|GetS1-2)))
      (Variables|Default|SetSide2 (Utilities|Array|MakeArray (Variables|Default|GetS2-3) (Variables|Default|GetS2-2) (Variables|Default|GetS2-4) (Variables|Default|GetS2-1)))
      (Variables|Default|SetSide3 (Utilities|Array|MakeArray (Variables|Default|GetS3-2) (Variables|Default|GetS3-4) (Variables|Default|GetS3-3) (Variables|Default|GetS3-1))))
    (:then_2
      (CallFunction|SpawnNacelle (Variables|Default|GetSide1))
      (CallFunction|SpawnNacelle (Variables|Default|GetSide2))
      (CallFunction|SpawnNacelle (Variables|Default|GetSide3)))))

(fn ConstructionScript)

(fn GetSlot
  (params (Index :type Integer) (Array :type Array%20of%20Child%20Actor%20Component%20Object%20References))
  (bind _asbp_slots_building (Utilities|Casting|CastToBP_SlotsBuilding (Variables|/Script/Engine.ChildActorComponent|GetChildActor (Utilities|Array|Get(acopy) Array Index)))
    (:then
      (return _asbp_slots_building))
    (:CastFailed
      (return 0))))

(fn IsSlotEmpty
  (params (Index :type Integer) (Array :type Array%20of%20Child%20Actor%20Component%20Object%20References))
  (Utilities|IsValid (Variables|/Game/Blueprints/Building/BP_SlotsBuilding.BP_SlotsBuilding_C|GetActorRef (CallFunction|GetSlot Index Array))
    (:Is%20Valid
      (Development|PrintString "Not Null")
      (return false))
    (:Is%20Not%20Valid
      (return true))))

(fn SpawnNacelle
  (params (ArrayNacelle :type Array%20of%20Child%20Actor%20Component%20Object%20References))
  (bind _indexlist (LocalVariables|GetIndexList))
  (Utilities|Set|Clear _indexlist)
  (while (< (Utilities|Set|Length _indexlist) 2)
    (Utilities|Set|Add (LocalVariables|GetIndexList) (Math|Random|RandomIntegerinRange 0 (- (Utilities|Array|Length ArrayNacelle) 1))))
  (bind _result (Utilities|Set|ToArray (LocalVariables|GetIndexList)))
  (for _array_element _result
    (Default|SetActorRef (CallFunction|GetSlot _array_element ArrayNacelle) (stale _returnvalue))
    (bind _returnvalue (Game|SpawnActorfromClass "/Game/Blueprints/Building/BP_Nacelle.BP_Nacelle_C" (Math|Transform|MakeTransform (.location (Transformation|GetWorldTransform (Variables|/Game/Blueprints/Building/BP_SlotsBuilding.BP_SlotsBuilding_C|GetArrow (CallFunction|GetSlot _array_element ArrayNacelle)))) (.rotation (Transformation|GetWorldTransform (Variables|/Game/Blueprints/Building/BP_SlotsBuilding.BP_SlotsBuilding_C|GetArrow (CallFunction|GetSlot _array_element ArrayNacelle)))) "1,1,1") "Undefined" 0 0))
    (Transformation|AttachComponentToComponent _returnvalue (Variables|Default|GetCylinder) "None" "KeepWorld" "KeepRelative" "KeepWorld" true)))