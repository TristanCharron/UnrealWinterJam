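; BP_BuildingSpawner is an actor that spawns BP_Building instances at a height that rises with a running count.
; BeginPlay calls Spawn once, which increments NbBuildingsLoaded and places a building at StartPoint's rotation and the BuildingScale.
; Its location is StartPoint raised by FirstBuilding's vertical bounds extent (half its height) times that count, so repeated Spawn calls step upward.
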(event EventBeginPlay
  (CallFunction|Spawn))

(event Collision|EventActorBeginOverlap
  (params (OtherActor :type Actor%20Object%20Reference)))

(event EventTick
  (params (DeltaSeconds :type Float%20%28single-precision%29)))

(fn ConstructionScript)

(fn Spawn
  (bind _startpoint (Variables|Default|GetStartPoint))
  (Variables|Default|SetNbBuildingsLoaded (+ (Variables|Default|GetNbBuildingsLoaded) 1))
  (Game|SpawnActorfromClass "/Game/Blueprints/Building/BP_Building.BP_Building_C" (Math|Transform|MakeTransform (+ (Transformation|GetWorldLocation _startpoint) (* (Math|Vector|MakeVector 0.0 0.0 (.z (.BoxExtent (Collision|GetActorBounds (Variables|Default|GetFirstBuilding) false)))) (Variables|Default|GetNbBuildingsLoaded))) (Transformation|GetWorldRotation _startpoint) (Variables|Default|GetBuildingScale)) "Undefined" 0 0))