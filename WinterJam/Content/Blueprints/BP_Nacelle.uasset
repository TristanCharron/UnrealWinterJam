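; BP_Nacelle is a platform actor that destroys itself after a FakeCharacter has stood on it long enough.
; Begin overlap with a FakeCharacter sets an occupancy flag, and end overlap with any actor clears it.
; While the flag is set, Tick drains NacelleTimer by a fixed per-frame step, making the lifetime frame-rate dependent.
; The timer never resets, so contact time accumulates across visits.
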(event EventBeginPlay)

(event Collision|EventActorBeginOverlap
  (params (OtherActor :type Actor%20Object%20Reference))
  (Utilities|Casting|CastToFakeCharacter OtherActor)
  (Variables|Default|SetisCharacterOnPlatform true))

(event Collision|EventActorEndOverlap
  (params (OtherActor :type Actor%20Object%20Reference))
  (Variables|Default|SetisCharacterOnPlatform false))

(event EventTick
  (params (DeltaSeconds :type Float%20%28single-precision%29))
  (Utilities|FlowControl|Sequence
    (:then_0
      (if (Variables|Default|GetisCharacterOnPlatform)
        (Variables|Default|SetNacelleTimer (- (Variables|Default|GetNacelleTimer) 0.05))
        (if (<= (Variables|Default|GetNacelleTimer) 0.0)
          (Actor|DestroyActor))))))

(fn ConstructionScript)