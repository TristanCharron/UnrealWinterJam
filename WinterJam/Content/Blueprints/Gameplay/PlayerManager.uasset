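; PlayerManager tracks the game's players and which of them are dead, to detect game over.
; It listens to the GameManager's game start dispatcher and, on In Game, runs Spawn, which clears the dead list, caches the CameraManager and appends existing PlayerBase actors to PlayerList without creating any.
; PlayerDeath and PlayerSaved add and remove dead players.
; When both lists match in length after a death, it only prints "GameOver".
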(event Custom|OnGameStart
  (params (NextGameState :type EGameStates%20Enum :default "NewEnumerator0"))
  (switch Utilities|FlowControl|Switch|SwitchonEGameStates NextGameState
    (:NewEnumerator1
      (CallFunction|Spawn))))

(event EventBeginPlay
  (EventDispatchers|BindEventtoGameStartDispatcher (CallFunction|GetGameManager) (delegate Custom|OnGameStart)))

(event Collision|EventActorBeginOverlap
  (params (OtherActor :type Actor%20Object%20Reference)))

(event EventTick
  (params (DeltaSeconds :type Float%20%28single-precision%29)))

(fn ConstructionScript)

(fn Spawn
  (Utilities|Array|Clear (Variables|Default|GetPlayerDeadList))
  (Variables|Default|SetCameraManager (CallFunction|GetCameraManager))
  (bind _outactors (Actor|GetAllActorsOfClass "/Game/Blueprints/Gameplay/PlayerBase.PlayerBase_C"))
  (for _array_element _outactors
    (Utilities|Array|Add (Variables|Default|GetPlayerList) _array_element)))

(fn PlayerDeath
  (params (Player :type Player%20Base%20Object%20Reference))
  (Utilities|Array|AddUnique (Variables|Default|GetPlayerDeadList) Player)
  (if (== (Utilities|Array|Length (Variables|Default|GetPlayerList)) (Utilities|Array|Length (Variables|Default|GetPlayerDeadList)))
    (Development|PrintString "GameOver")))

(fn PlayerSaved
  (params (Player :type Player%20Base%20Object%20Reference))
  (Utilities|Array|RemoveItem (Variables|Default|GetPlayerDeadList) Player))