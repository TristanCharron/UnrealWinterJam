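; Base player character for a side-view game with a right-stick-aimed tongue attack, jumping, cleaning for score and a placeholder spray.
; Input and tick start on the In Game state; a simple state variable accepts new actions only when idle.
; A timeline lerps the tongue outward, notifying overlapped IOverlappleByTongue actors.
; Leaving the rendered view triggers death, which notifies PlayerManager and immediately repositions the player at the camera's destination.
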(event Custom|OnGameStart
  (params (NextGameState :type EGameStates%20Enum :default "NewEnumerator0"))
  (switch Utilities|FlowControl|Switch|SwitchonEGameStates NextGameState
    (:NewEnumerator1
      (Variables|Default|SetCameraManager (CallFunction|GetCameraManager))
      (Input|EnableInput (Game|GetPlayerController (Variables|Input|GetPlayerID)))
      (bind _player_manager (CallFunction|GetPlayerManager))
      (Variables|Default|SetPlayerManager _player_manager)
      (CallFunction|SetMaterial)
      (Utilities|FlowControl|Delay 1.0)
      (Actor|Tick|SetActorTickEnabled true))))

(event Custom|ShootTongueEvent
  (Variables|Default|SetisShootingTongue true)
  (bind _alpha (Timeline|ShootTongueTimeline PlayFromStart)
    (:Update
      (Transformation|SetWorldLocation (Variables|Default|GetTongue) (Math|Vector|Lerp(Vector) (Tongue|GetStartTongueLocation) (Tongue|GetEndTongueLocation) _alpha) false false))
    (:Finished
      (Variables|Default|SetisShootingTongue false)
      (State|EndState))))

(event Custom|CleanEvent
  (Development|PrintString "I Clean")
  (Utilities|FlowControl|Delay 2.0)
  (CallFunction|OnCompleteClean))

(event EventBeginPlay
  (EventDispatchers|BindEventtoGameStartDispatcher (CallFunction|GetGameManager) (delegate Custom|OnGameStart)))

(event EventOnLanded
  (params (Hit :type Hit%20Result%20Structure%20%28by%20ref%29))
  (if (.bBlockingHit (Collision|BreakHitResult Hit))
    (if (Utilities|Enum|Equal(Enum) (Variables|Default|GetCurrentState) "NewEnumerator5")
      (State|EndState))))

(event EventTick
  (params (DeltaSeconds :type Float%20%28single-precision%29))
  (CallFunction|Aim)
  (if (not (Class|Actor|WasRecentlyRendered 1.0))
    (State|ChangeState "NewEnumerator4")))

(event Input|ActionEvents|InputActionAction_Jump
  (params (Key :type Key%20Structure))
  ;[1 1 1] Action Buttons
  (:Pressed
    (CallFunction|PressJump))
  (:Released
    (Character|StopJumping)))

(event Input|ActionEvents|InputActionAction_RightBumper
  (params (Key :type Key%20Structure))
  ;[1 1 1] Action Buttons
  (:Pressed
    (Input|Spray)))

(event Input|ActionEvents|InputActionAction_LeftBumper
  (params (Key :type Key%20Structure))
  ;[1 1 1] Action Buttons
  (:Pressed
    (Input|Clean)))

(event Input|ActionEvents|InputActionAction_RightTrigger
  (params (Key :type Key%20Structure))
  ;[1 1 1] Action Buttons
  (:Pressed
    (State|ChangeState "NewEnumerator2")))

(event Input|AxisEvents|InputAxisAxis_MoveRight
  (params (AxisValue :type Float%20%28single-precision%29))
  ;[1 1 1] Axis
  (Input|Move AxisValue)
  (Variables|Input|SetLeftStick_X AxisValue))

(event Input|AxisEvents|InputAxisAxis_CameraRight
  (params (AxisValue :type Float%20%28single-precision%29))
  ;[1 1 1] Axis
  (Variables|Input|SetRightStick_X AxisValue))

(event Input|AxisEvents|InputAxisAxis_CameraForward
  (params (AxisValue :type Float%20%28single-precision%29))
  ;[1 1 1] Axis
  (Variables|Input|SetRightStick_Y AxisValue))

(event OnComponentBeginOverlap(Tongue)
  (params (OverlappedComponent :type Primitive%20Component%20Object%20Reference) (OtherActor :type Actor%20Object%20Reference) (OtherComp :type Primitive%20Component%20Object%20Reference) (OtherBodyIndex :type Integer) (bFromSweep :type Boolean) (SweepResult :type Hit%20Result%20Structure%20%28by%20ref%29))
  (if (Utilities|DoesObjectImplementInterface OtherActor "/Game/Blueprints/Interfaces/IOverlappleByTongue.IOverlappleByTongue_C")
    (Class|IOverlapplebyTongue|OnBeginOverlap(Message) OtherActor)))

(fn ConstructionScript)

(fn Move
  (params (Input :type Float%20%28single-precision%29))
  (bind _mesh (Variables|Character|GetMesh))
  (bind _returnvalue (Transformation|GetWorldRotation _mesh))
  (Pawn|Input|AddMovementInput (Math|Vector|GetForwardVector (Pawn|GetControlRotation :!class /Script/Engine.Pawn)) Input false)
  (Transformation|SetWorldRotation _mesh (Math|Rotator|MakeRotator (.roll _returnvalue) (.pitch _returnvalue) (Math|Interpolation|FInterpTo (.yaw _returnvalue) (* (Math|Float|Sign(Float) Input) -9e+01) (Utilities|Time|GetWorldDeltaSeconds) 15.0)) false false))

(fn PressJump
  (Character|Jump)
  (State|ChangeState "NewEnumerator5"))

(fn Spray
  (Development|PrintString "I Spray"))

(fn Clean
  (CallFunction|CleanEvent))

(fn Aim
  (if (and (> (Math|Vector2D|Vector2DLength (Math|Vector2D|MakeVector2D (Variables|Input|GetRightStick_X) (Variables|Input|GetRightStick_Y))) 0.5) (not (Variables|Default|GetisShootingTongue)))
    (Transformation|SetWorldRotation (Variables|Default|GetTongueRotator) (Math|Rotator|MakeRotator 0.0 (CallFunction|GetAimAngle) 0.0) true false)))

(fn GetEndTongueLocation
  (return (+ (Transformation|GetActorLocation) (* (Math|Vector|GetForwardVector (Math|Rotator|FindLookatRotation (Transformation|GetActorLocation) (Transformation|GetWorldLocation (Variables|Default|GetTongue)))) (Variables|Default|GetTongueScale)))))

(fn ChangeState
  (params (NextState :type EPlayerState%20Enum :default "NewEnumerator3"))
  (if (Utilities|Enum|Equal(Enum) (Variables|Default|GetCurrentState) "NewEnumerator3")
    (Variables|Default|SetCurrentState NextState)
    (switch Utilities|FlowControl|Switch|SwitchonEPlayerState NextState
      (:NewEnumerator2
        (CallFunction|ShootTongueEvent))
      (:NewEnumerator4
        (CallFunction|Death)))))

(fn EndState
  (if (Utilities|Enum|NotEqual(Enum) (Variables|Default|GetCurrentState) "NewEnumerator3")
    (Variables|Default|SetCurrentState "NewEnumerator3")))

(fn Death
  (bind _cameramanager (Variables|Default|GetCameraManager))
  (bind _destinationcamera (Variables|/Game/Blueprints/Camera/CameraManager.CameraManager_C|GetDestinationCamera _cameramanager))
  (bind _returnvalue (Transformation|GetWorldLocation _destinationcamera))
  (Input|DisableInput (Game|GetPlayerController (Variables|Input|GetPlayerID)))
  (Default|PlayerDeath (Variables|Default|GetPlayerManager) self)
  (Development|PrintString "I am Dead")
  (Transformation|SetActorLocation (Math|Vector|MakeVector (.x _returnvalue) (Variables|/Game/Blueprints/Gameplay/PlayerManager.PlayerManager_C|GetPlayerYPosition (Variables|Default|GetPlayerManager)) (.z _returnvalue)) false false)
  (Input|EnableInput (Game|GetPlayerController 0))
  (Default|PlayerSaved (Variables|Default|GetPlayerManager) self)
  (State|EndState))

(fn OnCompleteClean
  (Math|Integer|IncrementInt (Variables|Default|GetcurrentScore)
    (:%20%20
      (Default|CleanScore (CallFunction|GetGameManager) self))))

(fn SetMaterial
  (Rendering|Material|SetMaterial (Variables|Character|GetMesh) 0 (Variables|Material|GetPlayerMaterial)))

(fn GetAimAngle
  (return (* (+ (Class|KismetMathLibrary|DegAtan2 (Variables|Input|GetRightStick_Y) (Variables|Input|GetRightStick_X)) 9e+01) -1.0)))

(fn GetStartTongueLocation
  (return (+ (Transformation|GetActorLocation) (* (Math|Vector|GetForwardVector (Math|Rotator|FindLookatRotation (Transformation|GetActorLocation) (Transformation|GetWorldLocation (Variables|Default|GetTongue)))) 1.8e+02))))