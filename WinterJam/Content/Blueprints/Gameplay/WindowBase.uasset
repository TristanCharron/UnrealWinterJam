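; WindowBase is a cleanable window actor that players interact with by standing in its box trigger.
; On BeginPlay it picks one of two window types at random, weighted toward the first.
; Box overlaps store or clear the current PlayerBase, printing a debug string on entry.
; GettingCleaned, not called within this graph, increments a timer per call, then marks the window clean and notifies that player at the threshold.
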(event OnComponentBeginOverlap(Box)
  (params (OverlappedComponent :type Primitive%20Component%20Object%20Reference) (OtherActor :type Actor%20Object%20Reference) (OtherComp :type Primitive%20Component%20Object%20Reference) (OtherBodyIndex :type Integer) (bFromSweep :type Boolean) (SweepResult :type Hit%20Result%20Structure%20%28by%20ref%29))
  (bind _asplayer_base (Utilities|Casting|CastToPlayerBase OtherActor))
  (Development|PrintString "coucou je uis frog")
  (Variables|Default|SetcurretnPlayer _asplayer_base))

(event OnComponentEndOverlap(Box)
  (params (OverlappedComponent :type Primitive%20Component%20Object%20Reference) (OtherActor :type Actor%20Object%20Reference) (OtherComp :type Primitive%20Component%20Object%20Reference) (OtherBodyIndex :type Integer))
  (Variables|Default|SetcurretnPlayer 0))

(event EventBeginPlay
  (switch int (Math|Random|RandomIntegerinRange 0 5)
    (:0
      (Variables|Default|Settype "NewEnumerator0" :!label _label))
    (:1
      (goto _label))
    (:2
      (goto _label))
    (:3
      (goto _label))
    (:4
      (Variables|Default|Settype "NewEnumerator1"))))

(event Collision|EventActorBeginOverlap
  (params (OtherActor :type Actor%20Object%20Reference)))

(event EventTick
  (params (DeltaSeconds :type Float%20%28single-precision%29)))

(fn ConstructionScript)

(fn GettingCleaned
  (Actor|Tick|SetActorTickEnabled (Variables|Default|GetisGettingCleaned))
  (Math|Float|IncrementFloat (Variables|Default|GetcleanTimer)
    (:%20%20
      (if (>= (Variables|Default|GetcleanTimer) (Variables|Default|GetmaxTimer))
        (Variables|Default|SetisClean true)
        (Variables|Default|SetisGettingCleaned false)
        (Variables|Default|SetcleanTimer 0.0)
        (Default|OnCompleteClean (Variables|Default|GetcurretnPlayer))))))