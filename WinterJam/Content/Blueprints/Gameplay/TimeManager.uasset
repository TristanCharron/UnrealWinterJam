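; TimeManager is the match countdown actor that shows the remaining time on a world text render and ends the game when time runs out.
; It listens to the game manager's start dispatcher, resets the time to the game length on entering In Game and enables tick.
; Tick moves the text to the main camera's height, decrements and displays the time, then disables itself and switches to EndGame at zero.
; It also exposes a clamped completion ratio.
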(event Custom|StartGame
  (params (CurrentGameState :type EGameStates%20Enum :default "NewEnumerator0"))
  (switch Utilities|FlowControl|Switch|SwitchonEGameStates CurrentGameState
    (:NewEnumerator1
      (Variables|Default|SetCurrentGameTime (Variables|Default|GetGameLength))
      (Actor|Tick|SetActorTickEnabled true))))

(event EventBeginPlay
  (EventDispatchers|BindEventtoGameStartDispatcher (CallFunction|GetGameManager) (delegate Custom|StartGame))
  (Variables|Default|SetCameraManager (CallFunction|GetCameraManager))
  (CallFunction|SetTimerTextRender 0.0))

(event EventTick
  (params (DeltaSeconds :type Float%20%28single-precision%29))
  (CallFunction|FollowCamera)
  (bind _istimeover (CallFunction|ChangeTime DeltaSeconds))
  (CallFunction|SetTimerTextRender (Variables|Default|GetCurrentGameTime))
  (if _istimeover
    (Actor|Tick|SetActorTickEnabled false)
    (Default|ChangeState (CallFunction|GetGameManager) "NewEnumerator2")))

(fn ConstructionScript)

(fn GetTimeCompletionRatio
  (return (Math|Float|Clamp(Float) (- 1.0 (/ (Variables|Default|GetCurrentGameTime) (Variables|Default|GetGameLength))))))

(fn FollowCamera
  (bind _timertextrender (Variables|Default|GetTimerTextRender))
  (bind _returnvalue (Transformation|GetActorLocation _timertextrender))
  (Transformation|SetActorLocation _timertextrender (Math|Vector|MakeVector (.x _returnvalue) (.y _returnvalue) (.z (Transformation|GetWorldLocation (Default|GetMainCamera (Variables|Default|GetCameraManager))))) false false))

(fn ChangeTime
  (params (Tick :type Float%20%28single-precision%29))
  (bind _output_get (Variables|Default|SetCurrentGameTime (- (Variables|Default|GetCurrentGameTime) Tick)))
  (return (<= _output_get 0.0)))

(fn SetTimerTextRender
  (params (Time :type Float%20%28single-precision%29))
  (bind _timertextrender (Variables|Default|GetTimerTextRender))
  (bind _textrender (Variables|/Script/Engine.TextRenderActor|GetTextRender _timertextrender))
  (if (<= Time 0.0)
    (Rendering|Components|TextRender|SetText _textrender (Utilities|Text|MakeLiteralText ""))
    (else
      (Rendering|Components|TextRender|SetText _textrender (Utilities|Text|MakeLiteralText (Utilities|Text|ToText(Float) Time "HalfToEven"))))))